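; Player controller base Blueprint that opens and closes the room selection build menu.
; OpenSelectBuildMenu creates a WBP_SelectRoom widget, stores it in UIBuildRef, adds it to the viewport and shows the mouse cursor.
; CloseSelectBuildMenu removes the stored widget from its parent but leaves the cursor visible.
; BeginPlay, Tick and the construction script are empty, and a disconnected duplicate of the widget creation never runs.
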(event `self.ReceiveBeginPlay`)

(event `self.OpenSelectBuildMenu`
  (bind _returnvalue (`|CreateWidget` "/Game/Assets/Blueprints/UI/Build/WBP_SelectRoom.WBP_SelectRoom_C" self))
  (bind _output_get (set `self.UIBuildRef` _returnvalue))
  (`UserWidget.AddToViewport` _output_get 10)
  (set `self.bShowMouseCursor` true))

(event `self.CloseSelectBuildMenu`
  (`Widget.RemoveFromParent` (`self.UIBuildRef`)))

(fn `UserConstructionScript`)