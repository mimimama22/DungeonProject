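; Dungeon path actor that lays a flattened, slightly lowered run of spline meshes along its spline at construction time.
; GeneratedSlinePath calls its parent version, clears the tracked SplineMeshArray, then adds segments stepped by LenghtMesh, shortening the last to the spline end.
; Segment tangents are clamped in size, and each end location is printed.
; An older TrackSpline-based version of the loop remains unconnected in the event graph.
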(fn `GeneratedSlinePath`
  (returns (ReturnValue :type Boolean))
  (locals (SplineLength :type "Float (single-precision)") (ActualDistance :type "Float (double-precision)") (EndSpline :type Boolean) (StartLocation :type "Vector Structure") (StartTangent :type "Vector Structure") (EndLocation :type "Vector Structure") (EndTangent :type "Vector Structure"))
  (bind _endlocation (`local.EndLocation`))
  (`parent.GeneratedSlinePath`)
  (`|ExecutionSequence`
    (:`then_0`
      (for _array_element (`self.SplineMeshArray`)
        (`ActorComponent.K2_DestroyComponent` _array_element))
      (`KismetArrayLibrary.Array_Clear` (`self.SplineMeshArray`)))
    (:`then_1`
      (set `local.SplineLength` (`SplineComponent.GetSplineLength` (`self.SplineComponent`)))
      (set `local.ActualDistance` 0.0)
      (while (and (< (`local.ActualDistance`) (`local.SplineLength`)) (not (`local.EndSpline`)))
        (set `local.StartLocation` (`SplineComponent.GetLocationAtDistanceAlongSpline` (`self.SplineComponent`) (`local.ActualDistance`) "Local"))
        (set `local.StartTangent` (`SplineComponent.GetTangentAtDistanceAlongSpline` (`self.SplineComponent`) (`local.ActualDistance`) "Local"))
        (bind _output_get (set `local.ActualDistance` (+ (`local.ActualDistance`) (* (`self.LenghtMesh`) 100.0))))
        (set `local.EndSpline` (> _output_get (`local.SplineLength`)))
        (set `local.ActualDistance` (select `bool` (`local.EndSpline`) :`false` (`local.ActualDistance`) :`true` (`local.SplineLength`) :!type "Float (double-precision)"))
        (set `local.EndLocation` (`SplineComponent.GetLocationAtDistanceAlongSpline` (`self.SplineComponent`) (`local.ActualDistance`) "Local"))
        (set `local.EndTangent` (`SplineComponent.GetTangentAtDistanceAlongSpline` (`self.SplineComponent`) (`local.ActualDistance`) "Local"))
        (bind _returnvalue (`AddComponent|NODE_AddSplineMeshComponent-1` :`RelativeTransform` (`KismetMathLibrary.MakeTransform` (0.0 0.0 -12.5) (struct) (1.0 1.0 0.1))))
        (`KismetArrayLibrary.Array_Add` (`self.SplineMeshArray`) _returnvalue)
        (`KismetSystemLibrary.PrintString` (`KismetStringLibrary.Conv_VectorToString` _endlocation))
        (`SplineMeshComponent.SetStartAndEnd` _returnvalue (`local.StartLocation`) (`KismetMathLibrary.ClampVectorSize` (`local.StartTangent`) 0.0 300.0) _endlocation (`KismetMathLibrary.ClampVectorSize` (`local.EndTangent`) 0.0 300.0) true))
      (return true))))

(fn `UserConstructionScript`
  (`self.GeneratedSlinePath`))